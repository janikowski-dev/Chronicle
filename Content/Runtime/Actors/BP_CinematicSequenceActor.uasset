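; Cinematic actor that plays branching dialogue as Level Sequences relative to its transform, with numbered player responses.
; Start and finish requests run behind screen fades.
; Transitions filtered by Chronicle rules end the cinematic, auto-continue, or show responses while a second sequence player loops.
; The chosen transition raises its callbacks and plays its sequence from that node's start frame; the construction script updates participant and camera previews.
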(event Custom|OnCinematicFinishRequired_Event
  ;[0.15 0.15 0.15 0.5] Add Finish Callback
  (bind _returnvalue (UserInterface|CreateWidget "/Chronicle/Runtime/Widgets/WBP_FadeScreen.WBP_FadeScreen_C"))
  (UserInterface|Viewport|AddtoViewport _returnvalue 0)
  (Default|Fadein _returnvalue)
  (Utilities|FlowControl|Delay 0.5)
  (Sequencer|Player|Stop (Variables|/Script/LevelSequence.LevelSequenceActor|GetSequencePlayer (Variables|Players|GetMainPlayer)) :!class /Script/MovieScene.MovieSceneSequencePlayer)
  (Default|CallOnCinematicFinished)
  (Default|FadeOut _returnvalue)
  (Widget|RemovefromParent _returnvalue))

(event Custom|OnCinematicStartRequired_Event
  ;[0.15 0.15 0.15 0.5] Add Start Callback
  (bind _returnvalue (UserInterface|CreateWidget "/Chronicle/Runtime/Widgets/WBP_FadeScreen.WBP_FadeScreen_C"))
  (UserInterface|Viewport|AddtoViewport _returnvalue 0)
  (Default|Fadein _returnvalue)
  (Utilities|FlowControl|Delay 0.5)
  (Flow|StartCinematic)
  (Default|FadeOut _returnvalue)
  (Widget|RemovefromParent _returnvalue))

(event Input|EnhancedActionEvents|EnhancedInputActionIA_Respond
  (params (ActionValue :type Float%20%28double-precision%29) (ElapsedSeconds :type Float%20%28double-precision%29) (TriggeredSeconds :type Float%20%28double-precision%29) (InputAction :type Input%20Action%20Object%20Reference :default "/Chronicle/Runtime/Input/IA_Respond.IA_Respond"))
  ;[0.15 0.15 0.15 0.5] Input Handling
  (Flow|TryReadingResponse ActionValue))

(event EventBeginPlay
  ;[0.15 0.15 0.15 0.5] Initialization
  (Setup|CachePlayers)
  (Setup|InitializePlayers)
  (Setup|InitializeInput)
  ;[0.15 0.15 0.15 0.5] Add Start Callback
  (EventDispatchers|BindEventtoOnCinematicStartRequired (delegate Custom|OnCinematicStartRequired_Event))
  ;[0.15 0.15 0.15 0.5] Add Finish Callback
  (EventDispatchers|BindEventtoOnCinematicFinishRequired (delegate Custom|OnCinematicFinishRequired_Event)))

(fn ConstructionScript
  (Class|ChronicleCinematicSequenceActor|UpdateParticipantsPreview (Variables|Default|GetParticipantsPreview))
  (Class|ChronicleCinematicSequenceActor|UpdateCamerasPreview (Variables|Default|GetCamerasPreview)))

(fn StartCinematic
  (bind _info (Variables|Setup|GetInfo))
  (bind (_sequencesbyid _entrysequenceid) (Utilities|Struct|BreakChronicle_DialogueInfo _info))
  (bind _value (Utilities|Map|Find _sequencesbyid _entrysequenceid))
  (bind _sequence (Utilities|Struct|BreakChronicle_SequenceInfo _value))
  (Utilities|LoadAssetBlocking _sequence)
  (Class|LevelSequenceActor|SetSequence (Variables|Players|GetMainPlayer) (Utilities|ResolveSoftReference _sequence))
  (Sequencer|Player|Play (Variables|/Script/LevelSequence.LevelSequenceActor|GetSequencePlayer (Variables|Players|GetMainPlayer)) :!class /Script/MovieScene.MovieSceneSequencePlayer)
  (Variables|Flow|SetSequenceId (Utilities|Struct|BreakChronicle_DialogueInfo (Variables|Setup|GetInfo)))
  (Default|CallOnCinematicStarted))

(fn CachePlayers
  (bind _aslevel_sequence_actor (Utilities|Casting|CastToLevelSequenceActor (Variables|/Script/Engine.ChildActorComponent|GetChildActor (Variables|Default|GetMainLevelSequenceActor))))
  (Variables|Players|SetMainPlayer _aslevel_sequence_actor)
  (bind _aslevel_sequence_actor_2 (Utilities|Casting|CastToLevelSequenceActor (Variables|/Script/Engine.ChildActorComponent|GetChildActor (Variables|Default|GetResponseLevelSequenceActor))))
  (Variables|Players|SetResponsePlayer _aslevel_sequence_actor_2))

(fn InitializePlayers
  (bind _mainplayer (Variables|Players|GetMainPlayer))
  (bind _sequenceplayer (Variables|/Script/LevelSequence.LevelSequenceActor|GetSequencePlayer _mainplayer))
  (EventDispatchers|BindEventtoOnPause _sequenceplayer (EventDispatchers|CreateEvent :!event ProceedAfterSequence))
  (EventDispatchers|BindEventtoOnPlay _sequenceplayer (EventDispatchers|CreateEvent :!event InitMainPlayer))
  (EventDispatchers|BindEventtoOnPlay (Variables|/Script/LevelSequence.LevelSequenceActor|GetSequencePlayer (Variables|Players|GetResponsePlayer)) (EventDispatchers|CreateEvent :!event InitResponsePlayer)))

(fn InitMainPlayer
  (bind _returnvalue (Transformation|GetActorTransform))
  (bind (_location _rotation) (Math|Transform|BreakTransform _returnvalue))
  (Class|ChronicleCinematicSequenceActor|OffsetSpawnableTransforms (Variables|Players|GetMainPlayer) _location _rotation))

(fn ProceedAfterSequence
  ;[0.15 0.15 0.15 0.5] Designate Transitions
  (Utilities|Array|Clear (Variables|Flow|GetAvailableTransitions))
  (for _array_element (Utilities|Struct|BreakChronicle_SequenceInfo (.Value (Utilities|Map|Find (Utilities|Struct|BreakChronicle_DialogueInfo (Variables|Setup|GetInfo)) (Variables|Flow|GetSequenceId))))
    (bind _returnvalue (Class|ChronicleRuleSubsystem|Resolve (Subsystems|GetChronicleRuleSubsystem) (Utilities|Struct|BreakChronicle_TransitionInfo _array_element)))
    (if _returnvalue
      (Utilities|Array|Add (Variables|Flow|GetAvailableTransitions) _array_element)))
  ;[0.15 0.15 0.15 0.5] Handle Transition To The Next Sequence (Or Gameplay)
  (if (or (Utilities|Array|IsEmpty (Variables|Flow|GetAvailableTransitions)) (Utilities|Enum|Equal(Enum) (Utilities|Struct|BreakChronicle_TransitionInfo (Utilities|Array|Get(acopy) (Variables|Flow|GetAvailableTransitions))) "Game"))
    (Default|CallOnCinematicFinishRequired)
    (Class|ChronicleCinematicSequenceActor|LockontheLastFrame (Variables|Players|GetMainPlayer))
    (Sequencer|Player|Pause (Variables|/Script/LevelSequence.LevelSequenceActor|GetSequencePlayer (Variables|Players|GetMainPlayer)))
    (Class|ChronicleSubtitleSubsystem|HideSubtitles (Subsystems|GetChronicleSubtitleSubsystem))
    (elif (Utilities|Enum|Equal(Enum) (Utilities|Struct|BreakChronicle_TransitionInfo (Utilities|Array|Get(acopy) (Variables|Flow|GetAvailableTransitions))) "AutoContinue")
      (Flow|ReadResponse)
      (else
        (for _array_element_2 (Variables|Flow|GetAvailableTransitions)
          (if (Utilities|Enum|Equal(Enum) (Utilities|Struct|BreakChronicle_TransitionInfo _array_element_2) "Response")
            (Utilities|Array|Add (LocalVariables|GetResponses) (Utilities|Text|FormatText "{Number}. {Content}" (+ (Utilities|Array|Length (LocalVariables|GetResponses)) 1) (Utilities|Struct|BreakChronicle_SequenceInfo (.Value (Utilities|Map|Find (Utilities|Struct|BreakChronicle_DialogueInfo (Variables|Setup|GetInfo)) (Utilities|Struct|BreakChronicle_TransitionInfo _array_element_2))))))))
        (Class|ChronicleSubtitleSubsystem|ShowResponses (Subsystems|GetChronicleSubtitleSubsystem) (LocalVariables|GetResponses))
        (Flow|StartReadingResponse)))))

(fn StartReadingResponse
  (Variables|Flow|SetIsAcceptingResponses true)
  (Class|MovieSceneSequencePlayer|PlayLooping (Variables|/Script/LevelSequence.LevelSequenceActor|GetSequencePlayer (Variables|Players|GetResponsePlayer)) -1)
  (Class|ChronicleCinematicSequenceActor|PlayDefaultIdleAnimations (Variables|Players|GetMainPlayer)))

(fn TryReadingResponse
  (params (ResponseIndex :type Float%20%28double-precision%29))
  (bind _returnvalue (Math|Float|Truncate ResponseIndex))
  (bind _returnvalue_2 (- _returnvalue 1))
  (if (and (Variables|Flow|GetIsAcceptingResponses) (< _returnvalue_2 (Utilities|Array|Length (Variables|Flow|GetAvailableTransitions))))
    (Flow|ReadResponse _returnvalue_2)
    (Variables|Flow|SetIsAcceptingResponses false)
    (Sequencer|Player|Stop (Variables|/Script/LevelSequence.LevelSequenceActor|GetSequencePlayer (Variables|Players|GetResponsePlayer)) :!class /Script/MovieScene.MovieSceneSequencePlayer)))

(fn ReadResponse
  (params (TransitionIndex :type Integer))
  (bind _info (Variables|Setup|GetInfo))
  (bind _availabletransitions (Variables|Flow|GetAvailableTransitions))
  (bind _sequencesbyid (Utilities|Struct|BreakChronicle_DialogueInfo _info))
  (bind _output (Utilities|Array|Get(acopy) _availabletransitions TransitionIndex))
  (bind (_callbacks _sequenceid) (Utilities|Struct|BreakChronicle_TransitionInfo _output))
  (bind (_sequenceid_2 _nodeid) (Utilities|Struct|BreakChronicle_TransitionInfo _output))
  (bind _value (Utilities|Map|Find _sequencesbyid _sequenceid_2))
  (bind _sequence (Utilities|Struct|BreakChronicle_SequenceInfo _value))
  (Utilities|LoadAssetBlocking _sequence)
  (Class|ChronicleRuleSubsystem|Raise (Subsystems|GetChronicleRuleSubsystem) _callbacks)
  (Class|LevelSequenceActor|SetSequence (Variables|Players|GetMainPlayer) (Utilities|ResolveSoftReference _sequence))
  (Class|ChronicleCinematicSequenceActor|SetPlaybackPosition (Variables|Players|GetMainPlayer) (.Value (Utilities|Map|Find (Utilities|Struct|BreakChronicle_SequenceInfo _value) _nodeid)))
  (Sequencer|Player|Play (Variables|/Script/LevelSequence.LevelSequenceActor|GetSequencePlayer (Variables|Players|GetMainPlayer)) :!class /Script/MovieScene.MovieSceneSequencePlayer)
  (Variables|Flow|SetSequenceId _sequenceid))

(fn InitResponsePlayer
  (bind _returnvalue (Transformation|GetActorTransform))
  (bind (_location _rotation) (Math|Transform|BreakTransform _returnvalue))
  (Class|ChronicleCinematicSequenceActor|OffsetResponseCamera (Variables|Players|GetResponsePlayer) (Variables|Setup|GetResponseCameraTransform) _location _rotation))

(fn InitializeInput
  (Input|AddMappingContext (PlayerController|LocalPlayerSubsystems|GetEnhancedInputLocalPlayerSubsystem (Game|GetPlayerController 0)) "/Chronicle/Runtime/Input/IMC_Chronicle.IMC_Chronicle" 0 "(bIgnoreAllPressedKeysUntilRelease=True,bForceImmediately=False,bNotifyUserSettings=False)"))